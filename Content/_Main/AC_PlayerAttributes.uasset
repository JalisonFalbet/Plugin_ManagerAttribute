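; Player attributes component that manages named stats with levels, current and max values, built from setup ranges or restored from save data.
; Value edits clamp to the level range, level changes rescale max, and buffs or debuffs offset max, optionally merging.
; Timed changes queue in a list that one shared looping timer applies per tick, stopping once empty.
; Event dispatchers report changes, full or empty states, levels, buffs and regen.
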(fn GetAttributeLevels
  (params (Attribute :type String))
  (bind _array_element (Utilities|Array|ForEachLoopwithBreak (Variables|Default|GetSetup%20Attributes) :!label _label)
    (:LoopBody
      (LocalVariables|SetLevels (.RangePerLevels (Utilities|Struct|BreakPA_Strc_AttributesSetup _array_element)))
      (if (Utilities|Enum|Equal(Enum) (.Name (Utilities|Struct|BreakPA_Strc_AttributesSetup _array_element)) Attribute)
        (LocalVariables|SetFound true)
        (goto _label Break)))
    (:Completed
      (if (LocalVariables|GetFound)
        (return true (LocalVariables|GetLevels))
        (else
          (Development|PrintString (Utilities|String|Append "PA | " Attribute "Not Found In List") true true "(R=1.000000,G=0.000000,B=0.000000,A=1.000000)" 1e+01)
          (return false 0))))))

(fn StartAttributes
  (params (SaveGame? :type Boolean) (Save%20Attributes :type Array%20of%20PA%20Strc%20Attributes%20Values%20Structures))
  (if SaveGame?
    (Variables|Default|SetAttributes Save%20Attributes)
    (for _array_element (Variables|Default|GetAttributes) :!label _label
      (Default|CallOnAttributeSetup (Utilities|Struct|BreakPA_Strc_AttributesValues _array_element) _array_element))
    (else
      ;[0 0 0 1 40] Create the Initial Atributes list if dont have a save game setup
      (if (not (Utilities|Array|IsEmpty (Variables|Default|GetSetup%20Attributes)))
        (for _array_element_2 (Variables|Default|GetSetup%20Attributes)
          (if (Utilities|Array|IsEmpty (.RangePerLevels (Utilities|Struct|BreakPA_Strc_AttributesSetup _array_element_2)))
            (Development|PrintString (Utilities|String|Append "PA | " (.Name (Utilities|Struct|BreakPA_Strc_AttributesSetup _array_element_2)) " | Range Wrong Configured ") :!label _label_2)
            (elif (<= (.x (Utilities|Array|Get(acopy) (.RangePerLevels (Utilities|Struct|BreakPA_Strc_AttributesSetup _array_element_2)))) (.y (Utilities|Array|Get(acopy) (.RangePerLevels (Utilities|Struct|BreakPA_Strc_AttributesSetup _array_element_2)))))
              (Utilities|Array|Add (Variables|Default|GetAttributes) (Utilities|Struct|MakePA_Strc_AttributesValues (.Name (Utilities|Struct|BreakPA_Strc_AttributesSetup _array_element_2)) 0 (.y (Utilities|Array|Get(acopy) (.RangePerLevels (Utilities|Struct|BreakPA_Strc_AttributesSetup _array_element_2)))) (select (.StartEmpty? (Utilities|Struct|BreakPA_Strc_AttributesSetup _array_element_2)) 0.0 (.y (Utilities|Array|Get(acopy) (.RangePerLevels (Utilities|Struct|BreakPA_Strc_AttributesSetup _array_element_2)))))))
              (else
                (goto _label_2)))))
        (goto _label)
        (else
          (Development|PrintString "PA | Dont Has Attribute Setup" true true "(R=1.000000,G=0.000000,B=0.000000,A=1.000000)" 1e+01))))))

(fn ModifyValue
  (params (Attribute :type String) (Math :type Enum_MathSelect%20Enum :default "NewEnumerator0") (Is%20Percent? :type Boolean) (Value :type Float%20%28double-precision%29) (Notify? :type Boolean))
  (LocalVariables|SetLocal_Name Attribute)
  (LocalVariables|SetLocal_Math Math)
  (LocalVariables|SetLocalValue (select Is%20Percent? (/ (* (Math|Float|Clamp(Float) (Math|Float|Absolute(Float) Value) 0.0 1e+02) (Utilities|Struct|BreakPA_Strc_AttributesValues (.Value (PAFunctions|GetAttributeValues Attribute)))) 1e+02) (Math|Float|Absolute(Float) Value)))
  (bind (_found_ _attribute_infos _attribute_index) (Setup|IsAttributeValid? (LocalVariables|GetLocal_Name)))
  (if _found_
    (LocalVariables|SetLocal_Attribute _attribute_infos)
    (LocalVariables|SetAttributeIndex _attribute_index)
    (LocalVariables|SetLevelInfo (.Values (Setup|VerifyAttributeLevel (LocalVariables|GetLocal_Name) (Utilities|Struct|BreakPA_Strc_AttributesValues (LocalVariables|GetLocal_Attribute)))))
    (switch Utilities|FlowControl|Switch|SwitchonEnum_MathSelect (LocalVariables|GetLocal_Math)
      (:NewEnumerator0
        ;[0 0 0] Increment attribute value if is valid
        (if (> (.MaxValue (Utilities|Struct|BreakPA_Strc_AttributesValues (LocalVariables|GetLocal_Attribute))) (.CurrentValue (Utilities|Struct|BreakPA_Strc_AttributesValues (LocalVariables|GetLocal_Attribute))))
          (if (>= (+ (.CurrentValue (Utilities|Struct|BreakPA_Strc_AttributesValues (LocalVariables|GetLocal_Attribute))) (LocalVariables|GetLocalValue)) (.MaxValue (Utilities|Struct|BreakPA_Strc_AttributesValues (LocalVariables|GetLocal_Attribute))))
            (bind _structout (Utilities|Struct|SetmembersinPA_Strc_AttributesValues (LocalVariables|GetLocal_Attribute) (.MaxValue (Utilities|Struct|BreakPA_Strc_AttributesValues (LocalVariables|GetLocal_Attribute)))))
            (Utilities|Array|SetArrayElem (Variables|Default|GetAttributes) (LocalVariables|GetAttributeIndex) _structout)
            (else
              (bind _structout_2 (Utilities|Struct|SetmembersinPA_Strc_AttributesValues (LocalVariables|GetLocal_Attribute) (+ (.CurrentValue (Utilities|Struct|BreakPA_Strc_AttributesValues (LocalVariables|GetLocal_Attribute))) (LocalVariables|GetLocalValue))))
              (Utilities|Array|SetArrayElem (Variables|Default|GetAttributes) (LocalVariables|GetAttributeIndex) _structout_2)))
          (if (== (Utilities|Struct|BreakPA_Strc_AttributesValues (LocalVariables|GetLocal_Attribute)) (.y (LocalVariables|GetLevelInfo)))
            (Default|CallOnAttributeFull (LocalVariables|GetLocal_Name)))
          (else
            (return false))))
      (:NewEnumerator1
        ;[0 0 0] Decrement Value if is valid
        (if (> (.CurrentValue (Utilities|Struct|BreakPA_Strc_AttributesValues (LocalVariables|GetLocal_Attribute))) (.x (LocalVariables|GetLevelInfo)))
          (if (<= (- (.CurrentValue (Utilities|Struct|BreakPA_Strc_AttributesValues (LocalVariables|GetLocal_Attribute))) (LocalVariables|GetLocalValue)) (.x (LocalVariables|GetLevelInfo)))
            (bind _structout_3 (Utilities|Struct|SetmembersinPA_Strc_AttributesValues (LocalVariables|GetLocal_Attribute) (.x (LocalVariables|GetLevelInfo))))
            (Utilities|Array|SetArrayElem (Variables|Default|GetAttributes) (LocalVariables|GetAttributeIndex) _structout_3)
            (else
              (bind _structout_4 (Utilities|Struct|SetmembersinPA_Strc_AttributesValues (LocalVariables|GetLocal_Attribute) (- (.CurrentValue (Utilities|Struct|BreakPA_Strc_AttributesValues (LocalVariables|GetLocal_Attribute))) (LocalVariables|GetLocalValue))))
              (Utilities|Array|SetArrayElem (Variables|Default|GetAttributes) (LocalVariables|GetAttributeIndex) _structout_4)))
          (if (== (Utilities|Struct|BreakPA_Strc_AttributesValues (LocalVariables|GetLocal_Attribute)) (.x (LocalVariables|GetLevelInfo)))
            (Default|CallOnAttributeEmpty (LocalVariables|GetLocal_Name)))
          (else
            (return false)))))
    (if Notify?
      (Default|CallOnAttributeChanged Attribute Math Value (LocalVariables|GetLocal_Attribute)))
    (return true)
    (else
      (return false))))

(fn ModifyLevel
  (params (Attribute :type String) (Math :type Enum_MathSelect%20Enum :default "NewEnumerator0") (Level%20Modify :type Integer) (AdjustAttribute? :type Boolean))
  (LocalVariables|SetLocalValue (Math|Integer|Absolute(Integer) Level%20Modify))
  (bind (_found_ _attribute_infos _attribute_index) (Setup|IsAttributeValid? Attribute))
  (if _found_
    (LocalVariables|SetLocal_Attribute _attribute_infos)
    (LocalVariables|SetAttributeIndex _attribute_index)
    (LocalVariables|SetLevelsSetup (.LevelList (Setup|GetAttributeLevels Attribute)))
    (switch Utilities|FlowControl|Switch|SwitchonEnum_MathSelect Math
      (:NewEnumerator0
        (bind _output_get (LocalVariables|SetNewLevel (+ (Utilities|Struct|BreakPA_Strc_AttributesValues (LocalVariables|GetLocal_Attribute)) (LocalVariables|GetLocalValue))))
        (if (<= (+ (Utilities|Struct|BreakPA_Strc_AttributesValues (LocalVariables|GetLocal_Attribute)) (LocalVariables|GetLocalValue)) (Utilities|Array|LastIndex (LocalVariables|GetLevelsSetup)))
          (bind _structout (Utilities|Struct|SetmembersinPA_Strc_AttributesValues (LocalVariables|GetLocal_Attribute) _output_get (+ (.y (Utilities|Array|Get(acopy) (LocalVariables|GetLevelsSetup) _output_get)) (.BuffValue (Utilities|Struct|BreakPA_Strc_AttributesValues (LocalVariables|GetLocal_Attribute)))) (select AdjustAttribute? (+ (.y (Utilities|Array|Get(acopy) (LocalVariables|GetLevelsSetup) _output_get)) (.BuffValue (Utilities|Struct|BreakPA_Strc_AttributesValues (LocalVariables|GetLocal_Attribute)))) (.CurrentValue (Utilities|Struct|BreakPA_Strc_AttributesValues (LocalVariables|GetLocal_Attribute))))))
          (Utilities|Array|SetArrayElem (Variables|Default|GetAttributes) (LocalVariables|GetAttributeIndex) _structout)
          (Default|CallOnAttributeLevelUp Attribute _output_get _structout)
          (else
            (return false))))
      (:NewEnumerator1
        (bind _output_get_2 (LocalVariables|SetNewLevel (- (Utilities|Struct|BreakPA_Strc_AttributesValues (LocalVariables|GetLocal_Attribute)) (LocalVariables|GetLocalValue))))
        (if (>= (- (Utilities|Struct|BreakPA_Strc_AttributesValues (LocalVariables|GetLocal_Attribute)) (LocalVariables|GetLocalValue)) 0)
          (bind _structout_2 (Utilities|Struct|SetmembersinPA_Strc_AttributesValues (LocalVariables|GetLocal_Attribute) _output_get_2 (+ (.y (Utilities|Array|Get(acopy) (LocalVariables|GetLevelsSetup) _output_get_2)) (.BuffValue (Utilities|Struct|BreakPA_Strc_AttributesValues (LocalVariables|GetLocal_Attribute)))) (select (> (.CurrentValue (Utilities|Struct|BreakPA_Strc_AttributesValues (LocalVariables|GetLocal_Attribute))) (+ (.y (Utilities|Array|Get(acopy) (LocalVariables|GetLevelsSetup) _output_get_2)) (.BuffValue (Utilities|Struct|BreakPA_Strc_AttributesValues (LocalVariables|GetLocal_Attribute))))) (+ (.y (Utilities|Array|Get(acopy) (LocalVariables|GetLevelsSetup) _output_get_2)) (.BuffValue (Utilities|Struct|BreakPA_Strc_AttributesValues (LocalVariables|GetLocal_Attribute)))) (.CurrentValue (Utilities|Struct|BreakPA_Strc_AttributesValues (LocalVariables|GetLocal_Attribute))))))
          (Utilities|Array|SetArrayElem (Variables|Default|GetAttributes) (LocalVariables|GetAttributeIndex) _structout_2)
          (Default|CallOnAttributeLevelDown Attribute _output_get_2 _structout_2)
          (else
            (return false)))))
    (else
      (return false))))

(fn ModifyValueforTime
  (params (Attribute :type String) (Math :type Enum_MathSelect%20Enum :default "NewEnumerator0") (IsPercent? :type Boolean) (Value :type Float%20%28double-precision%29) (LenghtTime :type Float%20%28double-precision%29) (Override? :type Boolean))
  (if Override?
    (PAFunctions|CancelModifyforTime Attribute true))
  (LocalVariables|SetLocal_LenghtTime (Math|Float|SnapToGrid(Float) LenghtTime (Variables|Default|GetTickLenght)))
  (Utilities|Array|Add (Variables|Default|GetTimersLists) (Utilities|Struct|MakePA_Strc_AttributesRegenTick Attribute Math (/ (* (select IsPercent? (/ (* Value (Utilities|Struct|BreakPA_Strc_AttributesValues (.Value (PAFunctions|GetAttributeValues Attribute)))) 1e+02) Value) (Variables|Default|GetTickLenght)) (LocalVariables|GetLocal_LenghtTime)) 0.0 (LocalVariables|GetLocal_LenghtTime)))
  (if (not (Variables|Default|GetModifierTimerActive?))
    (bind _returnvalue (Utilities|Time|SetTimerbyEvent (EventDispatchers|CreateEvent :!event TickModifyFunction) (Variables|Default|GetTickLenght) true))
    (Variables|Default|SetModifierTimer_Handle _returnvalue)
    (Variables|Default|SetModifierTimerActive? true)))

(fn TickModifyFunction
  (if (Utilities|Array|IsNotEmpty (Variables|Default|GetTimersLists))
    (for (_array_element _array_index) (Variables|Default|GetTimersLists)
      (bind _output_get (LocalVariables|SetArrayElement _array_element))
      (LocalVariables|SetArrayIndex _array_index)
      (if (or (> (.CurrentTime (Utilities|Struct|BreakPA_Strc_AttributesRegenTick _output_get)) (.Time (Utilities|Struct|BreakPA_Strc_AttributesRegenTick _output_get))) (Utilities|Select :Index (.Math (Utilities|Struct|BreakPA_Strc_AttributesRegenTick _output_get)) :NewEnumerator0 (>= (.CurrentValue (Utilities|Struct|BreakPA_Strc_AttributesValues (.Value (PAFunctions|GetAttributeValues (.Attribute (Utilities|Struct|BreakPA_Strc_AttributesRegenTick _output_get)))))) (.MaxValue (Utilities|Struct|BreakPA_Strc_AttributesValues (.Value (PAFunctions|GetAttributeValues (.Attribute (Utilities|Struct|BreakPA_Strc_AttributesRegenTick _output_get))))))) :NewEnumerator1 (== (.CurrentValue (Utilities|Struct|BreakPA_Strc_AttributesValues (.Value (PAFunctions|GetAttributeValues (.Attribute (Utilities|Struct|BreakPA_Strc_AttributesRegenTick _output_get)))))) 0.0)))
        (PAFunctions|CancelModifyforTime (Utilities|Struct|BreakPA_Strc_AttributesRegenTick (LocalVariables|GetArrayElement)) true)
        (if (Utilities|Array|IsEmpty (Variables|Default|GetTimersLists))
          (Variables|Default|SetModifierTimerActive? false)
          (Utilities|Time|ClearandInvalidateTimerbyHandle (Variables|Default|GetModifierTimer_Handle)))
        (else
          (bind _structout (Utilities|Struct|SetmembersinPA_Strc_AttributesRegenTick (LocalVariables|GetArrayElement) (Math|Float|Clamp(Float) (+ (.CurrentTime (Utilities|Struct|BreakPA_Strc_AttributesRegenTick _output_get)) (Variables|Default|GetTickLenght)) 0.0 (.Time (Utilities|Struct|BreakPA_Strc_AttributesRegenTick _output_get)))))
          (Utilities|Array|SetArrayElem (Variables|Default|GetTimersLists) (LocalVariables|GetArrayIndex) _structout)
          (PAFunctions|ModifyValue (.Attribute (Utilities|Struct|BreakPA_Strc_AttributesRegenTick (LocalVariables|GetArrayElement))) (.Math (Utilities|Struct|BreakPA_Strc_AttributesRegenTick (LocalVariables|GetArrayElement))) false (.ValuePerTick (Utilities|Struct|BreakPA_Strc_AttributesRegenTick (LocalVariables|GetArrayElement))) false)
          (Default|CallOnAttributeCountRegen (.Attribute (Utilities|Struct|BreakPA_Strc_AttributesRegenTick (LocalVariables|GetArrayElement))) (.Math (Utilities|Struct|BreakPA_Strc_AttributesRegenTick (LocalVariables|GetArrayElement))) (.CurrentTime (Utilities|Struct|BreakPA_Strc_AttributesRegenTick (LocalVariables|GetArrayElement))) (.Time (Utilities|Struct|BreakPA_Strc_AttributesRegenTick (LocalVariables|GetArrayElement))) (.Value (PAFunctions|GetAttributeValues (.Attribute (Utilities|Struct|BreakPA_Strc_AttributesRegenTick (LocalVariables|GetArrayElement)))))))))
    (else
      (Variables|Default|SetModifierTimerActive? false)
      (Utilities|Time|ClearandInvalidateTimerbyHandle (Variables|Default|GetModifierTimer_Handle)))))

(fn ClearAllModifierTimers
  (if (Utilities|Array|IsEmpty (Variables|Default|GetTimersLists))
    (return false)
    (else
      (Utilities|Array|Clear (Variables|Default|GetTimersLists))
      (Variables|Default|SetModifierTimerActive? false)
      (Utilities|Time|ClearandInvalidateTimerbyHandle (Variables|Default|GetModifierTimer_Handle))
      (Default|CallOnAttributeEndRegen "All")
      (return true))))

(fn CancelModifyforTime
  (params (Attribute :type String) (Notify? :type Boolean))
  (if (Utilities|Array|IsEmpty (Variables|Default|GetTimersLists))
    (return false)
    (else
      (for (_array_element _array_index) (Variables|Default|GetTimersLists)
        (if (Utilities|Enum|Equal(Enum) (Utilities|Struct|BreakPA_Strc_AttributesRegenTick _array_element) Attribute)
          (Utilities|Array|RemoveIndex (Variables|Default|GetTimersLists) _array_index)
          (if Notify?
            (Default|CallOnAttributeEndRegen Attribute))
          (LocalVariables|SetFound? true)))
      (return (LocalVariables|GetFound?)))))

(fn AddAttributeBuff
  (params (Attribute :type String) (Value :type Float%20%28double-precision%29) (Setup :type Enum_BuffDebuff%20Enum :default "NewEnumerator0") (Merge? :type Boolean))
  (bind (_value _index) (PAFunctions|GetAttributeValues Attribute))
  (LocalVariables|SetLocal_Values _value)
  (LocalVariables|SetLocal_Index _index)
  (bind _output_get (LocalVariables|SetBuffValue (Utilities|Select :Index Setup :NewEnumerator0 (Math|Float|Absolute(Float) Value) :NewEnumerator1 (* (Math|Float|Absolute(Float) Value) -1.0))))
  (if (== _output_get 0.0)
    (return false)
    (else
      ;[0 0 0 1 30] Apply Buff or Debuff | First check if you need to override the values, if yes, check if there is an override value, if any, the values ​​override is performed and then a new check is done if the result is 0.
      (if Merge?
        (if (!= (Utilities|Struct|BreakPA_Strc_AttributesValues (LocalVariables|GetLocal_Values)) 0.0)
          (bind _output_get_2 (LocalVariables|SetBuffValue (+ (Utilities|Struct|BreakPA_Strc_AttributesValues (LocalVariables|GetLocal_Values)) (LocalVariables|GetBuffValue))))
          (if (!= _output_get_2 0.0)
            _
            (else
              (bind _success (PAFunctions|RemoveAttributeBuff Attribute true))
              (return _success)))
          (else
            (bind (_success_2 _value_2) (PAFunctions|RemoveAttributeBuff Attribute true :!label _label))
            (if _success_2
              (LocalVariables|SetLocal_Values _value_2))))
        (else
          (goto _label)))
      (bind _structout (Utilities|Struct|SetmembersinPA_Strc_AttributesValues (LocalVariables|GetLocal_Values) (+ (LocalVariables|GetBuffValue) (- (.MaxValue (Utilities|Struct|BreakPA_Strc_AttributesValues (LocalVariables|GetLocal_Values))) (.BuffValue (Utilities|Struct|BreakPA_Strc_AttributesValues (LocalVariables|GetLocal_Values))))) (select (<= (.CurrentValue (Utilities|Struct|BreakPA_Strc_AttributesValues (LocalVariables|GetLocal_Values))) (+ (LocalVariables|GetBuffValue) (- (.MaxValue (Utilities|Struct|BreakPA_Strc_AttributesValues (LocalVariables|GetLocal_Values))) (.BuffValue (Utilities|Struct|BreakPA_Strc_AttributesValues (LocalVariables|GetLocal_Values)))))) (.CurrentValue (Utilities|Struct|BreakPA_Strc_AttributesValues (LocalVariables|GetLocal_Values))) (+ (LocalVariables|GetBuffValue) (- (.MaxValue (Utilities|Struct|BreakPA_Strc_AttributesValues (LocalVariables|GetLocal_Values))) (.BuffValue (Utilities|Struct|BreakPA_Strc_AttributesValues (LocalVariables|GetLocal_Values)))))) (LocalVariables|GetBuffValue)))
      (Utilities|Array|SetArrayElem (Variables|Default|GetAttributes) (LocalVariables|GetLocal_Index) _structout)
      (Default|CallOnAttributeBuffed Attribute _structout Setup)
      (return true))))

(fn RemoveAttributeBuff
  (params (Attribute :type String) (Notify? :type Boolean))
  (bind _output_get (LocalVariables|SetLocal_Values (.Value (PAFunctions|GetAttributeValues Attribute))))
  (if (!= (Utilities|Struct|BreakPA_Strc_AttributesValues _output_get) 0.0)
    (bind _structout (Utilities|Struct|SetmembersinPA_Strc_AttributesValues (LocalVariables|GetLocal_Values) (+ (.MaxValue (Utilities|Struct|BreakPA_Strc_AttributesValues (LocalVariables|GetLocal_Values))) (* (.BuffValue (Utilities|Struct|BreakPA_Strc_AttributesValues (LocalVariables|GetLocal_Values))) -1.0)) (select (<= (.CurrentValue (Utilities|Struct|BreakPA_Strc_AttributesValues (LocalVariables|GetLocal_Values))) (+ (.MaxValue (Utilities|Struct|BreakPA_Strc_AttributesValues (LocalVariables|GetLocal_Values))) (* (.BuffValue (Utilities|Struct|BreakPA_Strc_AttributesValues (LocalVariables|GetLocal_Values))) -1.0))) (.CurrentValue (Utilities|Struct|BreakPA_Strc_AttributesValues (LocalVariables|GetLocal_Values))) (+ (.MaxValue (Utilities|Struct|BreakPA_Strc_AttributesValues (LocalVariables|GetLocal_Values))) (* (.BuffValue (Utilities|Struct|BreakPA_Strc_AttributesValues (LocalVariables|GetLocal_Values))) -1.0))) 0.0))
    (Utilities|Array|SetArrayElem (Variables|Default|GetAttributes) (.Index (PAFunctions|GetAttributeValues (Utilities|Struct|BreakPA_Strc_AttributesValues (LocalVariables|GetLocal_Values)))) _structout)
    (if Notify?
      (Default|CallOnAttributeUnBuffed Attribute _structout))
    (return true (.Value (PAFunctions|GetAttributeValues (Utilities|Struct|BreakPA_Strc_AttributesValues (LocalVariables|GetLocal_Values)))))
    (else
      (return false ""))))

(fn GetAttributeValues
  (params (Attribute :type String))
  (bind (_array_element _array_index) (Utilities|Array|ForEachLoopwithBreak (Variables|Default|GetAttributes) :!label _label)
    (:LoopBody
      (if (Utilities|Enum|Equal(Enum) (Utilities|Struct|BreakPA_Strc_AttributesValues _array_element) Attribute)
        (Utilities|FlowControl|Sequence
          (:then_0
            (goto _label Break))
          (:then_1
            (return _array_element _array_index)))))))

(fn HasFreeAttribute
  (params (Attribute :type String) (Value%20Entry :type Float%20%28double-precision%29))
  (bind _value (PAFunctions|GetAttributeValues Attribute))
  (return (< Value%20Entry (.CurrentValue (Utilities|Struct|BreakPA_Strc_AttributesValues _value))) _value))

(fn VerifyAttributeLevel
  (params (Attribute :type String) (Level :type Integer))
  (bind _array_element (Utilities|Array|ForEachLoopwithBreak (Variables|Default|GetSetup%20Attributes) :!label _label)
    (:LoopBody
      (LocalVariables|SetLevels (.RangePerLevels (Utilities|Struct|BreakPA_Strc_AttributesSetup _array_element)))
      (if (Utilities|Enum|Equal(Enum) (.Name (Utilities|Struct|BreakPA_Strc_AttributesSetup _array_element)) Attribute)
        (LocalVariables|SetFound true)
        (goto _label Break)))
    (:Completed
      (if (LocalVariables|GetFound)
        (return true (Utilities|Array|Get(acopy) (LocalVariables|GetLevels) Level))
        (else
          (Development|PrintString (Utilities|String|Append "PA | " Attribute "Not Found In List") true true "(R=1.000000,G=0.000000,B=0.000000,A=1.000000)" 1e+01)
          (return false ""))))))

(fn GetAttributeLevel
  (params (Attribute :type String))
  (return (Utilities|Struct|BreakPA_Strc_AttributesValues (.Value (PAFunctions|GetAttributeValues Attribute))) (.LevelList (Setup|GetAttributeLevels Attribute))))

(fn IsAttributeValid?
  (params (Attribute :type String))
  (bind (_array_element _array_index) (Utilities|Array|ForEachLoopwithBreak (Variables|Default|GetAttributes) :!label _label)
    (:LoopBody
      (LocalVariables|SetAttributeIndex _array_index)
      (LocalVariables|SetInfo _array_element)
      (if (Utilities|Enum|Equal(Enum) (.AttributeName (Utilities|Struct|BreakPA_Strc_AttributesValues _array_element)) Attribute)
        (LocalVariables|SetFoundAttribute? true)
        (goto _label Break)))
    (:Completed
      (if (LocalVariables|GetFoundAttribute?)
        (return true (LocalVariables|GetInfo) (LocalVariables|GetAttributeIndex))
        (else
          (return false "" 0))))))